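; BP_PanoPoint is a panorama point actor that links to other points and visualizes those connections in the editor.
; Its construction script zeroes actor rotation, orients an arrow by height and default heading, then verifies connections, with a manual refresh toggle.
; VerifyConnections mirrors two-way links, promotes mutual one-way links and updates neighbors one level deep.
; Links appear as color-coded arrows aimed at their targets, while older spline-drawing code sits unused.
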(fn `AddConnectionSpline`
  (params (TargetPano :type "/Game/render_utils/BP/BP_PanoPoint Object Reference") (`2Way?` :type Boolean :default true))
  (locals (NewSpline :type "SplineComponent Object Reference") (NewArrow :type "ArrowComponent Object Reference"))
  (if (`self.Connections Visibility`)
    (`/Engine/EditorBlueprintResources/StandardMacros.IsValid` TargetPano
      (:`Is Valid`
        (bind _returnvalue (`AddComponent|NODE_AddArrowComponent-0` :`RelativeTransform` (`KismetMathLibrary.MakeTransform` (0.0 0.0 0.0))))
        (bind _output_get (set `local.NewArrow` _returnvalue))
        (`SceneComponent.K2_AttachToComponent` _output_get (`self.Arrow`) "None" "SnapToTarget" "KeepWorld" "SnapToTarget" false)
        (`ArrowComponent.SetArrowColor` (`local.NewArrow`) (select `bool` (`local.2Way?`) :`false` (struct :`R` 0.27195 :`G` 0.319485 :`B` 1.0 :`A` 1.0) :`true` (struct :`R` 1.0 :`G` 0.900066 :`B` 0.318365 :`A` 1.0) :!type "LinearColor Structure"))
        (`SceneComponent.K2_SetWorldRotation` (`local.NewArrow`) (`KismetMathLibrary.FindLookAtRotation` (`SceneComponent.K2_GetComponentLocation` (`self.Arrow`)) (`SceneComponent.K2_GetComponentLocation` (`/Game/render_utils/BP/BP_PanoPoint.Box` (`local.TargetPano`)))) false false)
        (set `ArrowComponent.ArrowLength` (* (`KismetMathLibrary.VSize` (- (`SceneComponent.K2_GetComponentLocation` (`self.Arrow`)) (`SceneComponent.K2_GetComponentLocation` (`/Game/render_utils/BP/BP_PanoPoint.Box` (`local.TargetPano`))))) 3.3) (`local.NewArrow`))))))

(fn `UserConstructionScript`
  (`|ExecutionSequence`
    (:`then_0`
      (`self.K2_SetActorRotation` :`self` self)
      (`SceneComponent.K2_SetRelativeLocation` (`self.Arrow`) (`KismetMathLibrary.MakeVector` 0.0 0.0 (`self.Height`)) false false)
      (bind _output_get (set `self.defaultRotation` (mod (+ (`self.defaultRotation`) 360.0) 360.0)))
      (`SceneComponent.K2_SetWorldRotation` (`self.Arrow`) (`KismetMathLibrary.MakeRotator` 0.0 0.0 _output_get) false true))
    (:`then_1`
      (`self.VerifyConnections` true :!label _label))
    (:`then_2`
      (if (`self.ManualRefresh`)
        (set `self.ManualRefresh` false)
        (goto _label)))))

(fn `VerifyConnections`
  (params (SelfInitiated :type Boolean))
  (`|ExecutionSequence`
    (:`then_0`
      (`KismetArrayLibrary.Array_Append` (`self.2WayConnectionSplines`) (`self.1WayConnectionSplines`))
      (for _array_element (`self.2WayConnectionSplines`)
        (`/Engine/EditorBlueprintResources/StandardMacros.IsValid` _array_element
          (:`Is Valid`
            (`ActorComponent.K2_DestroyComponent` _array_element))))
      (`KismetArrayLibrary.Array_Clear` (`self.2WayConnectionSplines`))
      (`KismetArrayLibrary.Array_Clear` (`self.1WayConnectionSplines`)))
    (:`then_1`
      (bind _result (`BlueprintSetLibrary.Set_ToArray` (`self.2WayConnections`)))
      (for _array_element_2 _result
        (`/Engine/EditorBlueprintResources/StandardMacros.IsValid` _array_element_2
          (:`Is Valid`
            (`|ExecutionSequence`
              (:`then_0`
                (`BlueprintSetLibrary.Set_Remove` (`self.1WayConnections`) _array_element_2))
              (:`then_1`
                (`self.AddConnectionSpline` _array_element_2))
              (:`then_2`
                (`BlueprintSetLibrary.Set_Add` (`/Game/render_utils/BP/BP_PanoPoint.2WayConnections` _array_element_2) self)
                (if (`local.SelfInitiated`)
                  (`self.VerifyConnections` _array_element_2 false))))))))
    (:`then_2`
      (bind _result_2 (`BlueprintSetLibrary.Set_ToArray` (`self.1WayConnections`)))
      (for _array_element_3 _result_2
        (`/Engine/EditorBlueprintResources/StandardMacros.IsValid` _array_element_3
          (:`Is Valid`
            (`self.AddConnectionSpline` _array_element_3 false)
            (if (`BlueprintSetLibrary.Set_Contains` (`/Game/render_utils/BP/BP_PanoPoint.1WayConnections` _array_element_3) self)
              (`BlueprintSetLibrary.Set_Add` (`/Game/render_utils/BP/BP_PanoPoint.2WayConnections` _array_element_3) self)
              (if (`local.SelfInitiated`)
                (`self.VerifyConnections` _array_element_3 false)))))))))