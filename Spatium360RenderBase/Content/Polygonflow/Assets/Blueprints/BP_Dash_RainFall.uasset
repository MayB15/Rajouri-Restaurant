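; Placeable rain effect actor from the Polygonflow Dash assets that exposes rainfall and fog settings as actor variables.
; The Construction Script pushes those variables into float parameters on the DashRainfall effect component, covering rain amount, velocity, tilt, spawn area, splash fog and distant fog look.
; The event graph holds only disabled stub events, so the actor has no runtime logic of its own.
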(fn `UserConstructionScript`
  (bind _dash_rainfall (`self.Dash_Rainfall`))
  (`NiagaraComponent.SetVariableFloat` _dash_rainfall "SpawnRate" (`self.Rain Amount`))
  (`NiagaraComponent.SetVariableFloat` _dash_rainfall "Fog_Density" (`self.Splash Fog Density`))
  (`NiagaraComponent.SetVariableFloat` _dash_rainfall "Fog_Hue" (`self.Fog Hue`))
  (`NiagaraComponent.SetVariableFloat` _dash_rainfall "Rain_Velocity" (`self.Rain Velocity`))
  (`NiagaraComponent.SetVariableFloat` _dash_rainfall "Spawn_Radius_X" (`self.Spawn Radius X`))
  (`NiagaraComponent.SetVariableFloat` _dash_rainfall "Spawn_Radius_Y" (`self.Spawn Radius Y`))
  (`NiagaraComponent.SetVariableFloat` _dash_rainfall "Fog_Brightness" (`self.Fog Brightness`))
  (`NiagaraComponent.SetVariableFloat` _dash_rainfall "Fog_Saturation" (`self.Fog Saturation`))
  (`NiagaraComponent.SetVariableFloat` _dash_rainfall "Distant_Fog_Amount" (`self.Distant Fog Amount`))
  (`NiagaraComponent.SetVariableFloat` _dash_rainfall "Distant_Fog_Density" (`self.Distant Fog Density`))
  (`NiagaraComponent.SetVariableFloat` _dash_rainfall "Distant_Fog_Radius" (`self.Distant Fog Radius`))
  (`NiagaraComponent.SetVariableFloat` _dash_rainfall "Distant_Fog_Hue" (`self.Distant Fog Hue`))
  (`NiagaraComponent.SetVariableFloat` _dash_rainfall "Distant_Fog_Saturation" (`self.Distant Fog Saturation`))
  (`NiagaraComponent.SetVariableFloat` _dash_rainfall "Distant_Fog_Spread" (`self.Distant Fog Spread`))
  (`NiagaraComponent.SetVariableFloat` _dash_rainfall "Rain_Tilt_Y" (`self.Tilt Rain Y Axes`)))