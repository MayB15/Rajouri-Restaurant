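; BP_Dash_Snowfall is a placeable snowfall effect that exposes snow, fog and wind settings for its SnowFall particle component.
; The Construction Script copies the Blueprint's variables into the component's float parameters, covering spawn rate, foreground and background fog, wind, turbulence and radii.
; The generically named SpawnRadius parameter is fed by BGFogSpawnRadius.
; The Event Graph holds only disabled placeholder events, so the Blueprint adds no runtime logic.
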(fn `UserConstructionScript`
  (bind _snowfall (`self.SnowFall`))
  (`NiagaraComponent.SetVariableFloat` _snowfall "SpawnRate" (`self.Snow Spawn Rate `))
  (`NiagaraComponent.SetVariableFloat` _snowfall "FGFogDensity" (`self.Foreground Fog Density`))
  (`NiagaraComponent.SetVariableFloat` _snowfall "BGFogDensity" (`self.Background Fog Density`))
  (`NiagaraComponent.SetVariableFloat` _snowfall "WindVelocity" (`self.Wind Velocity`))
  (`NiagaraComponent.SetVariableFloat` _snowfall "WindDirectionX" (`self.Wind Direction X`))
  (`NiagaraComponent.SetVariableFloat` _snowfall "WindDirectionY" (`self.Wind Direction Y`))
  (`NiagaraComponent.SetVariableFloat` _snowfall "Turbulance" (`self.Turbulance`))
  (`NiagaraComponent.SetVariableFloat` _snowfall "SpawnRadius" (`self.BG Fog Spawn Radius`))
  (`NiagaraComponent.SetVariableFloat` _snowfall "BGFogRadius" (`self.BG Fog Radius`)))